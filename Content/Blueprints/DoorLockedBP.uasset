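; Locked door actor that the third-person character can unlock, then swing open and closed.
; An outer Box marks the player as in range, while InnerBox marks them as able to unlock.
; ControlDoor first releases the Locker with physics and destroys it after a delay.
; Later calls alternate timed door rotations through a FlipFlop, ignored while moving, or print a locked message if still locked.
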(event OnComponentBeginOverlap(Box)
  (params (OverlappedComponent :type Primitive%20Component%20Object%20Reference) (OtherActor :type Actor%20Object%20Reference) (OtherComp :type Primitive%20Component%20Object%20Reference) (OtherBodyIndex :type Integer) (bFromSweep :type Boolean) (SweepResult :type Hit%20Result%20Structure%20%28by%20ref%29))
  ;[1 1 1] Control player position
  (Utilities|Casting|CastToThirdPersonCharacter OtherActor)
  (Variables|Default|SetisPlayerInRange true))

(event OnComponentEndOverlap(Box)
  (params (OverlappedComponent :type Primitive%20Component%20Object%20Reference) (OtherActor :type Actor%20Object%20Reference) (OtherComp :type Primitive%20Component%20Object%20Reference) (OtherBodyIndex :type Integer))
  ;[1 1 1] Control player position
  (Utilities|Casting|CastToThirdPersonCharacter OtherActor)
  (Variables|Default|SetisPlayerInRange false))

(event OnComponentBeginOverlap(innerBox)
  (params (OverlappedComponent :type Primitive%20Component%20Object%20Reference) (OtherActor :type Actor%20Object%20Reference) (OtherComp :type Primitive%20Component%20Object%20Reference) (OtherBodyIndex :type Integer) (bFromSweep :type Boolean) (SweepResult :type Hit%20Result%20Structure%20%28by%20ref%29))
  ;[1 1 1] Control player position
  (Utilities|Casting|CastToThirdPersonCharacter OtherActor)
  (Variables|Default|SetisPlayerAbleToUnlock true))

(event OnComponentEndOverlap(innerBox)
  (params (OverlappedComponent :type Primitive%20Component%20Object%20Reference) (OtherActor :type Actor%20Object%20Reference) (OtherComp :type Primitive%20Component%20Object%20Reference) (OtherBodyIndex :type Integer))
  ;[1 1 1] Control player position
  (Utilities|Casting|CastToThirdPersonCharacter OtherActor)
  (Variables|Default|SetisPlayerAbleToUnlock false))

(event EventControlDoor
  (bind _door (Variables|Default|Getdoor))
  (bind _locker (Variables|Default|GetLocker))
  (if (and (Variables|Default|GetisPlayerAbleToUnlock) (Variables|Default|GetisDoorLocked)) ; Is player able to unlock?
    (Variables|Default|SetisDoorLocked false) ; Set locked variable
    ;[1 1 1] Simulate Door Unlock
    (Physics|SetSimulatePhysics _locker true)
    (Utilities|FlowControl|Delay 2.0)
    (Components|DestroyComponent _locker)
    (else
      ;[1 1 1] Is player in Range, is door not moving and is the door not locked
      (if (and (Variables|Default|GetisPlayerInRange) (not (Variables|Default|GetisDoorMoving)))
        (if (Variables|Default|GetisDoorLocked)
          (Development|PrintString "Door is locked")
          (else
            ;[1 1 1] Rotating Door
            (Utilities|FlowControl|FlipFlop
              (:A
                (Variables|Default|SetisDoorMoving true)
                (Components|MoveComponentTo _door "0, 0, 0" "0,-125.000000, 0" false false 1.0 false) ; Open Door
                (Variables|Default|SetisDoorMoving false))
              (:B
                (Variables|Default|SetisDoorMoving true)
                (Components|MoveComponentTo _door "0, 0, 0" "0,0.000000, 0" false false 1.0 false) ; Close Door
                (Variables|Default|SetisDoorMoving false)))))))))

(fn ConstructionScript)