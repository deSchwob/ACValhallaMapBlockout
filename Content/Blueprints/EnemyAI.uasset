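; EnemyAI is an enemy Blueprint that walks a patrol route through up to four target actors, starting at BeginPlay.
; The AIonPatroul event nests AIMoveTo calls, checking each target's validity and advancing only on success.
; It restarts only when the third or fourth target is invalid.
; An invalid first or second target, any failed move, or completing the fourth move ends the patrol.
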(event Custom|AIonPatroul
  (bind _self self)
  (bind _target02 (Variables|Default|GetTarget02))
  (bind _target03 (Variables|Default|GetTarget03))
  (bind _target04 (Variables|Default|GetTarget04))
  (bind _target01 (Variables|Default|GetTarget01))
  (Utilities|IsValid _target01
    (:Is%20Valid
      (AI|AIMoveTo _self "0, 0, 0" _target01 5.0 false
        (:OnSuccess
          (Utilities|IsValid _target02
            (:Is%20Valid
              (AI|AIMoveTo _self "0,0.000000, 0" _target02 5.0 false
                (:OnSuccess
                  (Utilities|IsValid _target03
                    (:Is%20Valid
                      (AI|AIMoveTo _self "0, 0, 0" _target03 5.0 false
                        (:OnSuccess
                          (Utilities|IsValid _target04
                            (:Is%20Valid
                              (AI|AIMoveTo _self "0, 0, 0" _target04 5.0 false))
                            (:Is%20Not%20Valid
                              (CallFunction|AIonPatroul :!label _label))))))
                    (:Is%20Not%20Valid
                      (goto _label))))))))))))

(event EventBeginPlay
  (CallFunction|AIonPatroul))

(fn ConstructionScript)