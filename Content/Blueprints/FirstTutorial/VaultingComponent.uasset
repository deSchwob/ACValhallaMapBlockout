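; Actor component that lets the owning ThirdPersonCharacter vault onto ledges in front of it.
; While not vaulting, Tick traces down ahead of the capsule, checks ledge height, walkable slope and capsule clearance, and toggles a prompt widget.
; Calling Vault switches state, and Tick then lerps the character from its start to the cached landing point over VaultSpeed seconds.
; Debug drawing and height printing are left on.
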(event Custom|Vault
  (Variables|Private|SetProgress 0.0)
  (Variables|Private|SetStartingLocation (Transformation|GetActorLocation (Variables|Private|GetOwningCharacter)))
  (Variables|Private|SetVaultingState "NewEnumerator2"))

(event EventBeginPlay
  (bind _asthird_person_character (Utilities|Casting|CastToThirdPersonCharacter (Components|GetOwner)))
  (Variables|Private|SetOwningCharacter _asthird_person_character)
  (bind _returnvalue (UserInterface|CreateWidget "/Game/Blueprints/FirstTutorial/VaultWidget.VaultWidget_C" (.AsPlayer%20Controller (Utilities|Casting|CastToPlayerController (Pawn|GetController (Variables|Private|GetOwningCharacter))))))
  (Variables|Private|SetVaultWidget _returnvalue))

(event EventTick
  (params (DeltaSeconds :type Float%20%28single-precision%29))
  (Utilities|SwitchVaultingState
    (:NotVaulting
      (bind (_result _ending_location) (Public|CanVault))
      (if _result
        (Variables|Private|SetEnding%20Location _ending_location)
        (if (not (UserInterface|Viewport|IsinViewport (Variables|Private|GetVaultWidget)))
          (UserInterface|Viewport|AddtoViewport (Variables|Private|GetVaultWidget) 0))
        (elif (UserInterface|Viewport|IsinViewport (Variables|Private|GetVaultWidget))
          (Widget|RemovefromParent (Variables|Private|GetVaultWidget)))))
    (:Vaulting
      (Private|TickVault DeltaSeconds))))

(fn CanVault
  (bind _owningcharacter (Variables|Private|GetOwningCharacter))
  (bind _returnvalue (Transformation|GetActorLocation _owningcharacter))
  (bind _returnvalue_2 (Transformation|GetActorForwardVector _owningcharacter))
  (bind _returnvalue_3 (* _returnvalue_2 7e+01))
  (bind _returnvalue_4 (+ _returnvalue _returnvalue_3))
  (if (Utilities|Enum|Equal(Enum) (Variables|Private|GetVaultingState) "NewEnumerator0")
    (LocalVariables|SetCapsule%20%28local%29 (Variables|/Script/Engine.Character|GetCapsuleComponent (Variables|Private|GetOwningCharacter)))
    (bind (_outhit _returnvalue_5) (Collision|LineTraceByChannel (+ _returnvalue_4 (Math|Vector|MakeVector 0.0 0.0 (Components|Capsule|GetScaledCapsuleHalfHeight (LocalVariables|GetCapsule%20%28local%29)))) (- _returnvalue_4 (Math|Vector|MakeVector 0.0 0.0 (Components|Capsule|GetScaledCapsuleHalfHeight (LocalVariables|GetCapsule%20%28local%29)))) "TraceTypeQuery1" false (Utilities|Array|MakeArray (Variables|Private|GetOwningCharacter)) "ForOneFrame"))
    (if _returnvalue_5
      (bind (_result _ending_location) (Private|CanVaulttoHit (LocalVariables|GetCapsule%20%28local%29) _outhit))
      (return _result _ending_location)
      (else
        (return false "0, 0, 0")))
    (else
      (return false "0, 0, 0"))))

(fn CanVaulttoHit
  (params (Capsule :type Capsule%20Component%20Object%20Reference) (Hit :type Hit%20Result%20Structure))
  (bind _z (Math|Vector|BreakVector (.location Hit)))
  (bind _returnvalue (Components|Capsule|GetScaledCapsuleRadius Capsule))
  (bind _z_2 (Math|Vector|BreakVector (.traceend Hit)))
  (bind _returnvalue_2 (- _z _z_2))
  (Utilities|FlowControl|Sequence
    (:then_0
      ;[1 1 1] Make sure that the ledge is at an appropriate height
      (Development|PrintString (Utilities|String|ToString(Float) _returnvalue_2) true true "(R=0.000000,G=0.660000,B=1.000000,A=1.000000)" 0.0)
      (if (not (Math|Float|InRange(Float) _returnvalue_2 (Variables|Private|Constants|GetMinVaultingHeight) (Variables|Private|Constants|GetMaxVaultingHeight)))
        (return false "0, 0, 0")))
    (:then_1
      ;[1 1 1] Make sure the surface we are walking to is walkable
      (if (< (.Z (Math|Vector|BreakVector (.normal Hit))) (Class|CharacterMovementComponent|GetWalkableFloorZ (Variables|/Script/Engine.Character|GetCharacterMovement (Variables|Private|GetOwningCharacter))))
        (return false "0, 0, 0")))
    (:then_2
      ;[1 1 1] Make sure that there is enough room for us on top of the ledge
      (bind _output_get (LocalVariables|SetEndingLocation%20%28local%29 (+ (.location Hit) (Math|Vector|MakeVector 0.0 0.0 (Components|Capsule|GetScaledCapsuleHalfHeight Capsule)))))
      (bind _result (Private|CheckCapsuleCollision (+ _output_get (Math|Vector|MakeVector 0.0 0.0 _returnvalue)) (Components|Capsule|GetScaledCapsuleHalfHeight Capsule) _returnvalue true))
      (if _result
        (return false "0, 0, 0")))
    (:then_3
      (return true (LocalVariables|GetEndingLocation%20%28local%29)))))

(fn CheckCapsuleCollision
  (params (Center :type Vector) (HalfHeight :type Float%20%28single-precision%29) (Radius :type Float%20%28single-precision%29) (DrawDebug :type Boolean))
  (Utilities|FlowControl|Sequence
    (:then_0
      (if DrawDebug
        (Rendering|Debug|DrawDebugCapsule Center HalfHeight Radius "0, 0, 0" "(R=1.000000,G=1.000000,B=0.000000,A=1.000000)" 0.0 3.0)))
    (:then_1
      (bind _returnvalue (Collision|CapsuleOverlapActors Center Radius HalfHeight (Utilities|Array|MakeArray "ObjectTypeQuery1" "ObjectTypeQuery2" "ObjectTypeQuery4") "/Script/Engine.Actor" (Utilities|Array|MakeArray (Variables|Private|GetOwningCharacter))))
      (return _returnvalue))))

(fn TickVault
  (params (DeltaSeconds :type Float%20%28single-precision%29))
  (Utilities|FlowControl|Sequence
    (:then_0
      (Variables|Private|SetProgress (Math|Float|Clamp(Float) (+ (Variables|Private|GetProgress) (/ DeltaSeconds (Variables|Private|Constants|GetVaultSpeed))) 0.0))
      (Transformation|SetActorLocation (Variables|Private|GetOwningCharacter) (Math|Vector|Lerp(Vector) (Variables|Private|GetStartingLocation) (Variables|Private|GetEnding%20Location) (Variables|Private|GetProgress)) false true))
    (:then_1
      (if (>= (Variables|Private|GetProgress) 1.0)
        (Variables|Private|SetVaultingState "NewEnumerator0")))))