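; DoorBP is a door Blueprint that swings open and closed through a custom ControlDoor event.
; Box overlap events set and print IsPlayerInRange when a ThirdPersonCharacter enters or leaves.
; ControlDoor uses a FlipFlop to alternate one-second MoveComponentTo rotations, setting IsDoorMoving during each swing.
; It checks range and movement, but both branch outcomes reach the FlipFlop, so the check gates nothing.
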(event OnComponentBeginOverlap(Box)
  (params (OverlappedComponent :type Primitive%20Component%20Object%20Reference) (OtherActor :type Actor%20Object%20Reference) (OtherComp :type Primitive%20Component%20Object%20Reference) (OtherBodyIndex :type Integer) (bFromSweep :type Boolean) (SweepResult :type Hit%20Result%20Structure%20%28by%20ref%29))
  (Utilities|Casting|CastToThirdPersonCharacter OtherActor)
  (bind _output_get (Variables|Default|SetisPlayerInRange true))
  (Development|PrintString (Utilities|String|ToString(Boolean) _output_get)))

(event OnComponentEndOverlap(Box)
  (params (OverlappedComponent :type Primitive%20Component%20Object%20Reference) (OtherActor :type Actor%20Object%20Reference) (OtherComp :type Primitive%20Component%20Object%20Reference) (OtherBodyIndex :type Integer))
  (Utilities|Casting|CastToThirdPersonCharacter OtherActor)
  (bind _output_get (Variables|Default|SetisPlayerInRange false))
  (Development|PrintString (Utilities|String|ToString(Boolean) _output_get)))

(event EventBeginPlay)

(event Collision|EventActorBeginOverlap
  (params (OtherActor :type Actor%20Object%20Reference)))

(event EventTick
  (params (DeltaSeconds :type Float%20%28single-precision%29)))

(event EventControlDoor
  (bind _door (Variables|Default|Getdoor))
  (if (and (Variables|Default|GetisPlayerInRange) (not (Variables|Default|GetisDoorMoving)))
    _
    (else
      _))
  (Utilities|FlowControl|FlipFlop
    (:A
      (Variables|Default|SetisDoorMoving true)
      (Components|MoveComponentTo _door "0, 0, 0" "0,125.000000, 0" false false 1.0 false) ; Open Door
      (Variables|Default|SetisDoorMoving false))
    (:B
      (Variables|Default|SetisDoorMoving true)
      (Components|MoveComponentTo _door "0, 0, 0" "0,0.000000, 0" false false 1.0 false) ; Close Door
      (Variables|Default|SetisDoorMoving false))))

(fn ConstructionScript)